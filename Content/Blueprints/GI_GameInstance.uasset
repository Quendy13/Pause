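; GI_GameInstance is a game instance that sets up the persistent save object at startup.
; On Init it loads the BP_CustomSaveGame from a fixed slot into SaveGameRef, or creates a new one if none exists.
; A new save gets its AllCollectibles array filled with one entry per level, up to MaxLevels.
; The SaveGame event is empty and the SaveGameToSlot call is unconnected, so this graph never writes to disk.
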(event Custom|SaveGame)

(event EventInit
  (bind _returnvalue (SaveGame|DoesSaveGameExist "AllanChadPied"))
  (if _returnvalue
    (bind _returnvalue_2 (SaveGame|LoadGamefromSlot "AllanChadPied"))
    (bind _asbp_custom_save_game (Utilities|Casting|CastToBP_CustomSaveGame _returnvalue_2))
    (Variables|Default|SetSaveGameRef _asbp_custom_save_game)
    (else
      (bind _returnvalue_3 (SaveGame|CreateSaveGameObject "/Game/Blueprints/BP_CustomSaveGame.BP_CustomSaveGame_C"))
      (Variables|Default|SetSaveGameRef _returnvalue_3)
      (for _index (range 0 (- (Variables|Default|GetMaxLevels) 1))
        (Utilities|Array|Add :TargetArray (Variables|/Game/Blueprints/BP_CustomSaveGame.BP_CustomSaveGame_C|GetAllCollectibles (Variables|Default|GetSaveGameRef)))))))