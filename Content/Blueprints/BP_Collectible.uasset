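; BP_Collectible is a pickup actor that the third-person character collects by touching it.
; On Cube overlap it casts the other actor to BP_ThirdPersonCharacter, increments NbCollectible, adds itself to CollectiblesTable, sets IsCollected and destroys itself.
; Two unconnected chains that would re-credit the player from IsCollected or from a CollectiblesTable lookup never run.
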(event OnComponentBeginOverlap(Cube)
  (params (OverlappedComponent :type Primitive%20Component%20Object%20Reference) (OtherActor :type Actor%20Object%20Reference) (OtherComp :type Primitive%20Component%20Object%20Reference) (OtherBodyIndex :type Integer) (bFromSweep :type Boolean) (SweepResult :type Hit%20Result%20Structure%20%28by%20ref%29))
  (bind _asbp_third_person_character (Utilities|Casting|CastToBP_ThirdPersonCharacter OtherActor))
  (Math|Integer|IncrementInt (Variables|/Game/ThirdPerson/Blueprints/BP_ThirdPersonCharacter.BP_ThirdPersonCharacter_C|GetnbCollectible _asbp_third_person_character)
    (:%20%20
      (Utilities|Array|Add (Variables|/Game/ThirdPerson/Blueprints/BP_ThirdPersonCharacter.BP_ThirdPersonCharacter_C|GetCollectiblesTable _asbp_third_person_character) self)
      (Variables|Default|SetbIsCollected true)
      (Actor|DestroyActor))))

(event EventBeginPlay)

(fn ConstructionScript)